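; BP_WalkerUnit is an enemy unit Blueprint that randomly takes the simple Manny or Quinn skeletal mesh in its construction script.
; On interaction it plays a one-shot response animation on the mesh, then uses a retriggerable delay of the clip's length before restoring Animation Blueprint mode.
; Selecting the unit also switches the mesh back to Animation Blueprint mode if it is in another mode.
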(event EventInteractionBehavior
  (params (Interactor :type Strategy%20Unit%20Object%20Reference))
  (bind _response_animation (Variables|Default|GetResponse%20Animation))
  (Components|Animation|PlayAnimation (Variables|Character|GetMesh) _response_animation false)
  (Utilities|FlowControl|RetriggerableDelay (Animation|GetPlayLength _response_animation))
  (Components|Animation|SetAnimationMode (Variables|Character|GetMesh) "AnimationBlueprint" true))

(event EventUnitSelected
  (bind _mesh (Variables|Character|GetMesh))
  (if (Utilities|Enum|NotEqual(Enum) (Class|SkeletalMeshComponent|GetAnimationMode _mesh) "AnimationBlueprint")
    (Components|Animation|SetAnimationMode _mesh "AnimationBlueprint" true)))

(fn ConstructionScript
  (Components|SkeletalMesh|SetSkeletalMeshAsset (Variables|Character|GetMesh) (select (Math|Random|RandomBool) "/Game/Characters/Mannequins/Meshes/SKM_Manny_Simple.SKM_Manny_Simple" "/Game/Characters/Mannequins/Meshes/SKM_Quinn_Simple.SKM_Quinn_Simple")))